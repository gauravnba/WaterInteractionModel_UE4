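; BP_Cube is an actor that keyboard input nudges along the world axes, with a WaterPhysics component attached to it.
; Each press of the arrow keys (X and Y) or T and G (Z) applies one fixed-step swept SetActorLocation, with no continuous movement while held.
; The construction script assigns the Sphere component, despite the Cube name, as the mesh WaterPhysics uses.
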(event `Key|G`
  (params (Key :type "Key Structure" :default "AnyKey"))
  ;[1 1 1] Vertical movement
  (:`Pressed`
    (`self.K2_SetActorLocation` (`KismetMathLibrary.MakeVector` (.x (`self.K2_GetActorLocation`)) (.y (`self.K2_GetActorLocation`)) (+ (.z (`self.K2_GetActorLocation`)) -10.0)) true)))

(event `Key|T`
  (params (Key :type "Key Structure" :default "AnyKey"))
  ;[1 1 1] Vertical movement
  (:`Pressed`
    (`self.K2_SetActorLocation` (`KismetMathLibrary.MakeVector` (.x (`self.K2_GetActorLocation`)) (.y (`self.K2_GetActorLocation`)) (+ (.z (`self.K2_GetActorLocation`)) 10.0)) true)))

(event `Key|Right`
  (params (Key :type "Key Structure" :default "AnyKey"))
  ;[1 1 1] Lateral movement
  (:`Pressed`
    (`self.K2_SetActorLocation` (`KismetMathLibrary.MakeVector` (.x (`self.K2_GetActorLocation`)) (+ (.y (`self.K2_GetActorLocation`)) 10.0) (.z (`self.K2_GetActorLocation`))) true)))

(event `Key|Left`
  (params (Key :type "Key Structure" :default "AnyKey"))
  ;[1 1 1] Lateral movement
  (:`Pressed`
    (`self.K2_SetActorLocation` (`KismetMathLibrary.MakeVector` (.x (`self.K2_GetActorLocation`)) (+ (.y (`self.K2_GetActorLocation`)) -10.0) (.z (`self.K2_GetActorLocation`))) true)))

(event `Key|Up`
  (params (Key :type "Key Structure" :default "AnyKey"))
  ;[1 1 1] Longitunal movement
  (:`Pressed`
    (`self.K2_SetActorLocation` (`KismetMathLibrary.MakeVector` (+ (.x (`self.K2_GetActorLocation`)) 10.0) (.y (`self.K2_GetActorLocation`)) (.z (`self.K2_GetActorLocation`))) true)))

(event `Key|Down`
  (params (Key :type "Key Structure" :default "AnyKey"))
  ;[1 1 1] Longitunal movement
  (:`Pressed`
    (`self.K2_SetActorLocation` (`KismetMathLibrary.MakeVector` (+ (.x (`self.K2_GetActorLocation`)) -10.0) (.y (`self.K2_GetActorLocation`)) (.z (`self.K2_GetActorLocation`))) true)))

(fn `UserConstructionScript`
  (set `WaterPhysicsComponent.mMeshComponent` (`self.Sphere`) (`self.WaterPhysics`)))